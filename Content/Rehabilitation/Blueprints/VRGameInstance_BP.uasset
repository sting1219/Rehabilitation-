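; VR rehabilitation game instance that holds attempt and success counters, both reset on Init.
; NextTime advances the attempt count, capped one past TryCount, and reports whether that cap is reached.
; Success increments the success count, and GetRingScaleValue shrinks the ring scale per success up to GoalCount, with a minimum floor.
; Both counter updates print debug strings.
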(event Custom|Init
  (Variables|MapSetting|SetSuccessCount 0)
  (Variables|Default|SetCurrentCount 0))

(fn NextTime
  (bind _trycount (Variables|Default|GetTryCount))
  (bind _returnvalue (+ _trycount 1))
  (bind _output_get (Variables|Default|SetCurrentCount (Class|KismetMathLibrary|BMin (+ (Variables|Default|GetCurrentCount) 1) _returnvalue)))
  (Development|PrintString (Utilities|String|Append "Current Count : " (Utilities|String|ToString(Byte) _output_get)))
  (return (>= (Variables|Default|GetCurrentCount) _returnvalue)))

(fn Success
  (bind _output_get (Variables|MapSetting|SetSuccessCount (+ (Variables|MapSetting|GetSuccessCount) 1)))
  (Development|PrintString (Utilities|String|Append "Success Count : " (Utilities|String|ToString(Byte) _output_get))))

(fn GetRingScaleValue
  (bind _output_get (LocalVariables|SetLocalCalcValue (Class|KismetMathLibrary|BMin (Variables|MapSetting|GetSuccessCount) (Variables|GameSetting|GetGoalCount))))
  (return (Math|Float|Max(Float) (- (Variables|GameSetting|GetRing_Base_Scale_Value) (* (Math|Conversions|ToFloat(Byte) _output_get) (Variables|GameSetting|GetRing_Scale_Decrease_Value))) 0.1)))