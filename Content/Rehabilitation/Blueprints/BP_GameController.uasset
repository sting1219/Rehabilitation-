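; BP_GameController runs the rehabilitation game's ball-and-ring loop, placing both relative to a player position.
; A looping timer spawns grabbable balls at a spawn point and starts each moving toward the player position.
; It keeps a single ring, rotated to face the player position and created on BeginPlay.
; The GoalRing event replaces that ring after a short delay, destroying the old one before spawning the next.
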(event Custom|SpawnRing
  (bind _ringposition (Variables|Default|GetRingPosition))
  (bind _returnvalue (Transformation|GetWorldLocation _ringposition))
  (bind _ringobject (Variables|Default|GetRingObject)
    (:then
      (Actor|DestroyActor _ringobject))
    (:else
      _))
  (bind _returnvalue_2 (Game|SpawnActorfromClass "/Game/Rehabilitation/Blueprints/BP_Ring.BP_Ring_C" (Math|Transform|MakeTransform _returnvalue (Math|Rotator|FindLookatRotation _returnvalue (Transformation|GetWorldLocation (Variables|Default|GetPlayerPosition))) "1,1,1") "AlwaysSpawn" self 0))
  (Variables|Default|SetRingObject _returnvalue_2))

(event Custom|SpawnBall
  (bind _returnvalue (Game|SpawnActorfromClass "/Game/Rehabilitation/Blueprints/BP_Grabbable_Ball.BP_Grabbable_Ball_C" (Math|Transform|MakeTransform (Transformation|GetWorldLocation (Variables|Default|GetBallSpawnPosition)) "0, 0, 0" "1.000000,1.000000,1.000000") "AlwaysSpawn" self 0))
  (Default|MoveStart _returnvalue (Transformation|GetWorldLocation (Variables|Default|GetPlayerPosition))))

(event EventBeginPlay
  (Utilities|Time|SetTimerbyEvent (delegate Custom|SpawnBall) 5.0 true)
  (CallFunction|SpawnRing))

(event Collision|EventActorBeginOverlap
  (params (OtherActor :type Actor%20Object%20Reference)))

(event EventTick
  (params (DeltaSeconds :type Float%20%28single-precision%29)))

(event EventGoalRing
  (Utilities|FlowControl|Delay 1.0)
  (CallFunction|SpawnRing))

(fn ConstructionScript)