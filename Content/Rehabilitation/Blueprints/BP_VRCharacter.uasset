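; BP_VRCharacter is a character Blueprint that carries a VRPawn through a Child Actor component and keeps it at the character's location.
; BeginPlay caches that pawn as VRPawnBP, sets the character as its owner, and snap-attaches it to the character when no head-mounted display is enabled.
; Tick copies only the character's location to the pawn, leaving rotation independent of this update.
; Unconnected leftover nodes hold a controller lookup and a full-transform sync.
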(event EventBeginPlay
  (bind _asvrpawn (Utilities|Casting|CastToVRPawn (Variables|/Script/Engine.ChildActorComponent|GetChildActor (Variables|Default|GetChildActor))))
  (bind _output_get (Variables|Default|SetVRPawn%20BP _asvrpawn))
  (Actor|SetOwner _output_get self)
  (if (not (Class|HeadMountedDisplayFunctionLibrary|IsHeadMountedDisplayEnabled))
    (Transformation|AttachActorToActor _output_get self "root" "SnapToTarget" "SnapToTarget" "SnapToTarget" false)))

(event Collision|EventActorBeginOverlap
  (params (OtherActor :type Actor%20Object%20Reference)))

(event EventTick
  (params (DeltaSeconds :type Float%20%28single-precision%29))
  (bind _vrpawn_bp (Variables|Default|GetVRPawn%20BP)
    (:then
      (Transformation|SetActorLocation _vrpawn_bp (Transformation|GetActorLocation) false false))
    (:else)))

(fn ConstructionScript)