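; Grabbable ball for the rehabilitation game that glides toward a goal position until it is grabbed or arrives.
; MoveStart stores a target 75 units above the given goal and enables a Tick VInterpTo move, which destroys the ball once it is within range.
; Grabbed stops that movement, while TestThrow passes a velocity to the grab component's TryRelease to test throwing.
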(event Custom|MoveStart
  (params (goalposition :type Vector))
  (Variables|Default|SetIsEnable true)
  (Variables|Default|SetGoalPosition (+ goalposition "0, 0,75.000000")))

(event Custom|TestThrow
  (params (velocity :type Vector))
  (Default|TryRelease (Variables|Default|GetGrabComponent_Ball) velocity))

(event EventBeginPlay)

(event Collision|EventActorBeginOverlap
  (params (OtherActor :type Actor%20Object%20Reference)))

(event EventTick
  (params (DeltaSeconds :type Float%20%28single-precision%29))
  (bind _returnvalue (Transformation|GetActorLocation))
  (bind _goalposition (Variables|Default|GetGoalPosition))
  (if (Variables|Default|GetIsEnable)
    (Transformation|SetActorLocation (Math|Interpolation|VInterpTo _returnvalue _goalposition DeltaSeconds (Variables|Default|Getspeed)) false false)
    (if (<= (Math|Vector|Distance(Vector) _returnvalue _goalposition) 25.0)
      (Actor|DestroyActor))))

(event EventGrabbed
  (Variables|Default|SetIsEnable false))

(fn ConstructionScript)