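; BP_Ring is a goal ring that scores when a BP_Grabbable_Ball passes out through its underside.
; When the ball stops overlapping the Cylinder, a direction check confirms it is level with or below the ring's origin, then fires Goal.
; Goal plays an explosion and confirmation sound, prints a debug message, sets a short lifespan and notifies every BP_GameController.
; An alternative SpawnSystemAtLocation effect remains unconnected.
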(event OnComponentEndOverlap(Cylinder)
  (params (OverlappedComponent :type Primitive%20Component%20Object%20Reference) (OtherActor :type Actor%20Object%20Reference) (OtherComp :type Primitive%20Component%20Object%20Reference) (OtherBodyIndex :type Integer))
  (bind _asbp_grabbable_ball (Utilities|Casting|CastToBP_Grabbable_Ball OtherActor))
  (if (<= (.Z (Math|Vector|BreakVector (Math|Vector|GetUnitDirection(Vector) (Transformation|GetActorLocation) (Transformation|GetActorLocation _asbp_grabbable_ball)))) 0.0)
    (CallFunction|Goal)))

(event Custom|Goal
  (bind _returnvalue (Transformation|GetActorLocation))
  (Effects|SpawnEmitteratLocation "/Game/ExampleContent/Blueprint_Communication/Effects/P_Explosion_Fireball.P_Explosion_Fireball" _returnvalue)
  (Audio|SpawnSoundatLocation "/Engine/VREditor/Sounds/VR_confirm_Cue.VR_confirm_Cue" _returnvalue "0, 0, 0" 1.0 1.0 0.0 0 0)
  (Development|PrintString "goal")
  (Actor|SetLifeSpan 0.5)
  (bind _outactors (Actor|GetAllActorsOfClass "/Game/Rehabilitation/Blueprints/BP_GameController.BP_GameController_C"))
  (for _array_element _outactors
    (Class|BPIController|GoalRing(Message) _array_element)))

(event EventBeginPlay)

(event Collision|EventActorBeginOverlap
  (params (OtherActor :type Actor%20Object%20Reference)))

(event EventTick
  (params (DeltaSeconds :type Float%20%28single-precision%29)))

(fn ConstructionScript)