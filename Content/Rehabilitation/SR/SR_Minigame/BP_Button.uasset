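; Physical push button for the SR rehabilitation minigame, pressed by a BP_Finger actor entering its box.
; While tracking, Tick projects finger movement since contact onto the mesh's up vector, sinking the mesh by that absolute, clamped distance.
; At maximum travel it sends ButtonPressedMessage to its parent actor.
; Full press or the finger leaving starts an interpolated return, which blocks new tracking until the mesh is back at its origin.
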(event OnComponentBeginOverlap(Box)
  (params (OverlappedComponent :type Primitive%20Component%20Object%20Reference) (OtherActor :type Actor%20Object%20Reference) (OtherComp :type Primitive%20Component%20Object%20Reference) (OtherBodyIndex :type Integer) (bFromSweep :type Boolean) (SweepResult :type Hit%20Result%20Structure%20%28by%20ref%29))
  (if (and (not (Variables|Default|GetIsTracking)) (not (Variables|Default|GetIsReturning)))
    (bind _asbp_finger (Utilities|Casting|CastToBP_Finger OtherActor))
    (Variables|Default|SetAs%20BPFInger _asbp_finger)
    (Variables|Default|SetIsTracking true)
    (Variables|Default|SetHandOriginLocation (Transformation|GetActorLocation (Variables|Default|GetAs%20BPFInger)))
    (Variables|Default|SetBtnOriginLocation (Transformation|GetWorldLocation (Variables|Default|GetButtonMesh)))))

(event OnComponentEndOverlap(Box)
  (params (OverlappedComponent :type Primitive%20Component%20Object%20Reference) (OtherActor :type Actor%20Object%20Reference) (OtherComp :type Primitive%20Component%20Object%20Reference) (OtherBodyIndex :type Integer))
  (bind _asbp_finger (Utilities|Casting|CastToBP_Finger OtherActor))
  (if (== _asbp_finger (Variables|Default|GetAs%20BPFInger))
    (Variables|Default|SetIsTracking false)
    (Variables|Default|SetIsReturning true)))

(event Custom|FullyPressed
  (Variables|Default|SetIsTracking false)
  (Variables|Default|SetIsReturning true)
  (Class|BPIButtonPressed|ButtonPressed(Message) (Actor|GetParentActor)))

(event EventBeginPlay)

(event Collision|EventActorBeginOverlap
  (params (OtherActor :type Actor%20Object%20Reference)))

(event EventTick
  (params (DeltaSeconds :type Float%20%28single-precision%29))
  (if (Variables|Default|GetIsTracking)
    (Variables|Default|SetCurrentTravel (Math|Float|Clamp(Float) (Math|Float|Absolute(Float) (Math|Vector|VectorLength (Math|Vector|ProjectVectorontoVector (- (Transformation|GetActorLocation (Variables|Default|GetAs%20BPFInger)) (Variables|Default|GetHandOriginLocation)) (Math|Vector|GetUpVector (Variables|Default|GetButtonMesh))))) 0.0 (Variables|Default|GetMaximumTravel)))
    (bind _output_get (Variables|Default|SetBtnCurrentLocation (- (Variables|Default|GetBtnOriginLocation) (* (Math|Vector|GetUpVector (Variables|Default|GetButtonMesh)) (Variables|Default|GetCurrentTravel)))))
    (Transformation|SetWorldLocation (Variables|Default|GetButtonMesh) _output_get false false)
    (if (>= (Variables|Default|GetCurrentTravel) (Variables|Default|GetMaximumTravel))
      (CallFunction|FullyPressed))
    (elif (Variables|Default|GetIsReturning)
      (bind _output_get_2 (Variables|Default|SetBtnCurrentLocation (Math|Interpolation|VInterpTo (Variables|Default|GetBtnCurrentLocation) (Variables|Default|GetBtnOriginLocation) DeltaSeconds (Variables|Default|GetBtnInterpSpeed))))
      (Transformation|SetWorldLocation (Variables|Default|GetButtonMesh) _output_get_2 false false)
      (if (Class|KismetMathLibrary|EqualExactlyVectorVector (Variables|Default|GetBtnCurrentLocation) (Variables|Default|GetBtnOriginLocation))
        (Variables|Default|SetIsReturning false)))))

(fn ConstructionScript)